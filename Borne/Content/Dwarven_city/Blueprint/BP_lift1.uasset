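; Player-operated lift for the Dwarven city, with gears that turn as it moves.
; A Box trigger enables the first player's input while a Character overlaps it and disables it on exit.
; E plays and Q reverses a timeline that lerps the lift's relative location between StartPoint and EndPoint.
; Each update also rolls four gear meshes by GearRotation, with the same sign in both travel directions.
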(event `self.Box.OnComponentBeginOverlap`
  (params (OverlappedComponent :type "PrimitiveComponent Object Reference") (OtherActor :type "Actor Object Reference") (OtherComp :type "PrimitiveComponent Object Reference") (OtherBodyIndex :type Integer) (bFromSweep :type Boolean) (SweepResult :type "HitResult Structure (by ref)"))
  (cast `Character` OtherActor)
  (`self.EnableInput` (`GameplayStatics.GetPlayerController` 0)))

(event `Key|E`
  (params (Key :type "Key Structure"))
  (bind _gear_rotation (`self.Gear Rotation`))
  (:`Pressed`
    (bind (_direction _newtrack_0) (`Timeline|Timeline_1` :!label _label)
      (:`Update`
        (`SceneComponent.K2_SetRelativeLocation` (`self.Lift`) (`KismetMathLibrary.VLerp` (`self.Start point`) (`self.End point`) _newtrack_0) false false)
        (`SceneComponent.K2_AddLocalRotation` (`self.SM_gear`) (`KismetMathLibrary.MakeRotator` _gear_rotation) false false)
        (`SceneComponent.K2_AddLocalRotation` (`self.SM_gear1`) (`KismetMathLibrary.MakeRotator` _gear_rotation) false false)
        (`SceneComponent.K2_AddLocalRotation` (`self.SM_gear4`) (`KismetMathLibrary.MakeRotator` _gear_rotation) false false)
        (`SceneComponent.K2_AddLocalRotation` (`self.SM_gear3`) (`KismetMathLibrary.MakeRotator` _gear_rotation) false false)))))

(event `Key|Q`
  (params (Key :type "Key Structure"))
  (:`Pressed`
    (goto _label :!via `Reverse`)))

(event `self.Box.OnComponentEndOverlap`
  (params (OverlappedComponent :type "PrimitiveComponent Object Reference") (OtherActor :type "Actor Object Reference") (OtherComp :type "PrimitiveComponent Object Reference") (OtherBodyIndex :type Integer))
  (cast `Character` OtherActor)
  (`self.DisableInput` (`GameplayStatics.GetPlayerController` 0)))

(fn `UserConstructionScript`)