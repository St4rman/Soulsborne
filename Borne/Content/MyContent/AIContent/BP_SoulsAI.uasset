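; BP_SoulsAI is a boss AI character Blueprint that reports its health to the player's HUD.
; UpdateHealth finds the BorneCharacter and passes Health and MaxHealth to its PlayerHUD as boss health.
; Tick, marked temporary debug, derives RunDir from movement velocity and actor rotation.
; Tick also looks up BorneCharacter each frame, but the distance check on that result is unused.
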(event `self.ReceiveBeginPlay`)

(event `self.ReceiveTick`
  (params (DeltaSeconds :type "Float (single-precision)"))
  ;[0 0 0 0.5] THIS IS TEMPORARY/ DEBUG
  (`|ExecutionSequence`
    (:`then_0`
      (bind _returnvalue (`GameplayStatics.GetActorOfClass` "/Script/Borne.BorneCharacter")))
    (:`then_1`
      (set `self.RunDir` (`KismetAnimationLibrary.CalculateDirection` (`MovementComponent.Velocity` (`self.CharacterMovement`)) (`self.K2_GetActorRotation`))))))

(event `self.UpdateHealth`
  ;[0 0 0] update player hud
  (bind _returnvalue (`GameplayStatics.GetActorOfClass` "/Script/Borne.BorneCharacter"))
  (`SHUDComponent.SetBossHealth` (`BorneCharacter.PlayerHUD` _returnvalue) (`self.Health`) (`self.MaxHealth`)))

(fn `UserConstructionScript`)