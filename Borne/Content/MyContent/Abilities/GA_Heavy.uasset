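; GA_Heavy is a gameplay ability, apparently a placeholder for a heavy attack, that only prints a debug string and ends immediately on activation.
; Its activation check requires the owner to be a BorneCharacter with a valid equipped weapon from its InventoryComponent and no montage playing on its mesh.
; A PlayMontage node is left unconnected and never runs, and the CurrentWpn variable is unused.
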(event `self.K2_ActivateAbility`
  (`KismetSystemLibrary.PrintString` "Hello" true false (struct :`R` 1.0 :`B` 0.097865 :`A` 1.0) 1.0)
  (`self.K2_EndAbility`))

(fn `K2_CanActivateAbility`
  (params (ActorInfo :type "GameplayAbilityActorInfo Structure") (Handle :type "GameplayAbilitySpecHandle Structure"))
  (returns (RelevantTags :type "GameplayTagContainer Structure") (ReturnValue :type Boolean))
  (bind _asborne_character (cast `BorneCharacter` ActorInfo_OwnerActor)
    (:`then`
      (`/Engine/EditorBlueprintResources/StandardMacros.IsValid` (`SInventoryComponent.GetCurrentEquippedWeapon` (`BorneCharacter.InventoryComponent` _asborne_character))
        (:`Is Valid`
          (if (`AnimInstance.Montage_IsPlaying` (`SkeletalMeshComponent.GetAnimInstance` (`Character.Mesh` _asborne_character)) null)
            _
            (else
              (return (struct) true))))
        (:`Is Not Valid`
          _)))
    (:`CastFailed`
      _))
  (return (struct) false))