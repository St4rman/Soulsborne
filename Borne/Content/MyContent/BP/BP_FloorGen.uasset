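; BP_FloorGen is a procedural floor generator that tiles a room-sized area with mesh instances.
; The construction script divides RoomVector's X and Y by Dimension and truncates the results into grid counts.
; Nested loops add an instance to Floor at each grid point, spaced by Dimension along X and Y.
; The event graph holds only empty default events, so nothing runs during play.
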(fn `UserConstructionScript`
  (locals (Width :type Integer :default 0) (Depth :type Integer :default 0) (DIndex :type Integer) (wIndex :type Integer))
  (bind _dimension (`self.Dimension`))
  (bind _output_get (set `local.Width` (`KismetMathLibrary.FTrunc` (/ (.x (`self.RoomVector`)) _dimension))))
  (set `local.Depth` (`KismetMathLibrary.FTrunc` (/ (.y (`self.RoomVector`)) _dimension)))
  (for _index (range (+ _output_get 1))
    (set `local.wIndex` _index)
    (for _index_2 (range (+ (`local.Depth`) 1))
      (set `local.DIndex` _index_2)
      (`InstancedStaticMeshComponent.AddInstance` (`self.Floor`) (`KismetMathLibrary.MakeTransform` (`KismetMathLibrary.MakeVector` (`KismetMathLibrary.Conv_IntToDouble` (* (`local.wIndex`) (`self.Dimension`))) (`KismetMathLibrary.Conv_IntToDouble` (* (`local.DIndex`) (`self.Dimension`))))) false))))