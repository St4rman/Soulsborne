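; AC_Flask is a component that lets the player drink a limited-use healing flask.
; DoFlask proceeds only if the ASC owns none of the blocking gameplay tags, charges remain and no drink is already running.
; It spends a charge, shows the flask mesh and plays the drinking montage.
; After a delay of half the returned montage length, it applies GE_Heal through GAS, hides the mesh and clears the busy flag.
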(event `DoFlask`
  (params (ASC :type "AbilitySystemComponent Object Reference") (Player :type "Character Object Reference") (`Flask Mesh` :type "SceneComponent Object Reference"))
  (bind _flaskcount (`self.FlaskCount`))
  (if (not (`BlueprintGameplayTagLibrary.HasAnyTags` (`BlueprintGameplayTagLibrary.GetOwnedGameplayTags` ASC) (`self.GameplayTags`)))
    (if (and (> _flaskcount 0.0) (not (`self.IsFlasking`)))
      (set `self.FlaskCount` (- _flaskcount 1.0))
      (set `self.IsFlasking` true)
      (`SceneComponent.SetVisibility` `Flask Mesh` true false)
      (bind _returnvalue (`Character.PlayAnimMontage` Player "/Game/MyContent/Anims/AM_Drinking.AM_Drinking" 1.5 "StartFlask"))
      (`KismetSystemLibrary.Delay` (* _returnvalue 0.5))
      (`AbilitySystemComponent.BP_ApplyGameplayEffectToSelf` :`self` ASC :`GameplayEffectClass` "/Game/MyContent/GAS/Effects/OneShots/GE_Heal.GE_Heal_C")
      (`SceneComponent.SetVisibility` `Flask Mesh` false false)
      (set `self.IsFlasking` false))))