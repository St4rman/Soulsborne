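; Debug interaction actor that shows a weapon prompt widget while something overlaps its sphere.
; BeginPlay passes the actor's damage, stamina, texture and name variables into the WVP_WpnPrompt held by its widget component.
; Sphere begin and end overlap events toggle the widget's visibility, with no filter on the overlapping actor.
; The construction script sets a test name on the prompt, alongside a disconnected SetValues call with placeholder data.
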(event `self.ReceiveBeginPlay`
  (bind _aswvp_wpn_prompt (cast `/Game/MyContent/UI/WVP_WpnPrompt` (`WidgetComponent.GetWidget` (`self.Widget`))))
  (`/Game/MyContent/UI/WVP_WpnPrompt.SetValues` _aswvp_wpn_prompt (`self.Damage`) (`self.Stamina`) (`self.texture2d`) (`self.Name`)))

(event `self.Sphere.OnComponentBeginOverlap`
  (params (OverlappedComponent :type "PrimitiveComponent Object Reference") (OtherActor :type "Actor Object Reference") (OtherComp :type "PrimitiveComponent Object Reference") (OtherBodyIndex :type Integer) (bFromSweep :type Boolean) (SweepResult :type "HitResult Structure (by ref)"))
  (`SceneComponent.SetVisibility` (`self.Widget`) true false))

(event `self.Sphere.OnComponentEndOverlap`
  (params (OverlappedComponent :type "PrimitiveComponent Object Reference") (OtherActor :type "Actor Object Reference") (OtherComp :type "PrimitiveComponent Object Reference") (OtherBodyIndex :type Integer))
  (`SceneComponent.SetVisibility` (`self.Widget`) false false))

(fn `UserConstructionScript`
  (bind _aswvp_wpn_prompt (cast `/Game/MyContent/UI/WVP_WpnPrompt` (`WidgetComponent.GetWidget` (`self.Widget`))))
  (set `/Game/MyContent/UI/WVP_WpnPrompt.TextNameSet` "test" _aswvp_wpn_prompt))