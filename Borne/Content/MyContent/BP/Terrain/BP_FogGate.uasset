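; Souls-like fog gate that carries the player through into a boss fight.
; On overlap it drops collision, motion-warps the character to a target point with a slowed montage, and animates the fog's dynamic material Blend on a timeline.
; After the montage's duration, it restores model blocking without re-enabling the trigger, recolors the fog, tells the Souls AI controller to begin fighting and calls the player's boss visibility function.
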(event `self.ReceiveBeginPlay`
  (bind _plane (`self.Plane`))
  (bind _returnvalue (`PrimitiveComponent.CreateDynamicMaterialInstance` _plane 0 (`PrimitiveComponent.GetMaterial` _plane 0) "None"))
  (bind _output_get (set `self.Mat Ref` _returnvalue))
  (`MaterialInstanceDynamic.SetVectorParameterValue` _output_get "Color" (struct :`R` 10.0 :`G` 7.0 :`A` 1.0)))

(event `self.Box.OnComponentBeginOverlap`
  (params (OverlappedComponent :type "PrimitiveComponent Object Reference") (OtherActor :type "Actor Object Reference") (OtherComp :type "PrimitiveComponent Object Reference") (OtherBodyIndex :type Integer) (bFromSweep :type Boolean) (SweepResult :type "HitResult Structure (by ref)"))
  (bind _mat_ref (`self.Mat Ref`))
  (bind _asbp_third_person_character (cast `/Game/ThirdPerson/Blueprints/BP_ThirdPersonCharacter` OtherActor))
  (`PrimitiveComponent.SetCollisionEnabled` (`self.Box`) "NoCollision")
  (`PrimitiveComponent.SetCollisionEnabled` (`self.Model`) "NoCollision")
  (`BorneCharacter.MotionWarpOnFogGate` _asbp_third_person_character (`KismetMathLibrary.TransformLocation` (`self.GetTransform`) (`self.TeleportLocation`)))
  (`|ExecutionSequence`
    (:`then_0`
      (bind _returnvalue (`Character.PlayAnimMontage` _asbp_third_person_character "/Game/MyContent/Anims/Action/AM_FogGate.AM_FogGate" 0.5 "None"))
      (`KismetSystemLibrary.Delay` _returnvalue)
      (`|ExecutionSequence`
        (:`then_0`
          (`self.StartFIght`))
        (:`then_1`
          (`PrimitiveComponent.SetCollisionEnabled` (`self.Box`) "PhysicsOnly")
          (`PrimitiveComponent.SetCollisionEnabled` (`self.Model`) "QueryAndPhysics"))
        (:`then_2`
          (`MaterialInstanceDynamic.SetScalarParameterValue` _mat_ref "Blend" 1.0)
          (`MaterialInstanceDynamic.SetVectorParameterValue` _mat_ref "Color" (struct :`R` 0.285417 :`G` 0.199511 :`B` 0.230936 :`A` 1.0)))))
    (:`then_1`
      (bind (_direction _newtrack_0) (`Timeline|Timeline`)
        (:`Update`
          (`MaterialInstanceDynamic.SetScalarParameterValue` (`self.Mat Ref`) "Blend" (- 1.0 _newtrack_0)))))))

(event `StartFIght`
  (`|ExecutionSequence`
    (:`then_0`
      (bind _returnvalue (`GameplayStatics.GetActorOfClass` "/Game/MyContent/AIContent/Data/BP_SoulsAIController.BP_SoulsAIController_C"))
      (`/Game/MyContent/AIContent/Data/BP_SoulsAIController.BeginFight` _returnvalue))
    (:`then_1`
      (bind _returnvalue_2 (`GameplayStatics.GetActorOfClass` "/Game/ThirdPerson/Blueprints/BP_ThirdPersonCharacter.BP_ThirdPersonCharacter_C"))
      (`/Game/ThirdPerson/Blueprints/BP_ThirdPersonCharacter.SetBossVisiblity` _returnvalue_2))))

(fn `UserConstructionScript`)