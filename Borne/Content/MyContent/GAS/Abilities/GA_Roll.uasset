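; GA_Roll is a Gameplay Ability that makes the third-person character dodge, either rolling or backstepping.
; On activation it checks the cost and that the character is not falling, then commits the cost, otherwise it ends.
; With last movement input it applies pre-dodge rotation and plays the roll montage; without, a temporary backstep montage.
; Either montage resets the mesh to the character and ends the ability, only on completion.
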(event `self.K2_ActivateAbility`
  (bind _ownerplayer (`self.OwnerPlayer`))
  (bind _owningmesh (`self.OwningMesh`))
  (bind _asbp_third_person_character (cast `/Game/ThirdPerson/Blueprints/BP_ThirdPersonCharacter` (`.OwnerActor` (break `GameplayAbilityActorInfo` (`self.GetActorInfo`)))))
  (set `self.OwnerPlayer` _asbp_third_person_character)
  (set `self.OwningMesh` (`Character.Mesh` _asbp_third_person_character))
  (bind _returnvalue (`self.K2_CheckAbilityCost`))
  (if (and _returnvalue (not (`NavMovementComponent.IsFalling` (`Character.CharacterMovement` _asbp_third_person_character))))
    (`self.K2_CommitAbilityCost` false)
    (bind _returnvalue_2 (`HelperBPLib.HasLastMovementInput` _ownerplayer))
    (if _returnvalue_2
      (`HelperBPLib.AddRotationPreDodge` _ownerplayer)
      (`|PlayMontage` _owningmesh "/Game/MyContent/Anims/AM_Roll.AM_Roll"
        (:`OnCompleted`
          _))
      (else
        (`|PlayMontage` _owningmesh "/Game/MyContent/Anims/AM_TempBackstep.AM_TempBackstep"
          (:`OnCompleted`
            _))))
    (`HelperBPLib.ResetMeshToCharacter` (`self.OwnerPlayer`))
    (`self.K2_EndAbility`)
    (else
      (`self.K2_EndAbility`))))

(fn `NewFunction`)